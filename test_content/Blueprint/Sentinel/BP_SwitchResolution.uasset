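; Sentinel test Blueprint that profiles performance across the supported fullscreen resolutions.
; On test init it caches the resolution list, binds NextShot to the performance component's screenshot-finished event and profiles run 0 without changing resolution.
; Each NextShot increments the index, applies that resolution through GameUserSettings and starts profiling under an index-based name.
; The test finishes when the index leaves the list.
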(event Custom|NextShot
  (bind _resolutions (Variables|Default|GetResolutions))
  (bind _resolutionindex (Variables|Default|GetResolutionIndex))
  (bind _returnvalue (Utilities|String|ToString(Integer) _resolutionindex))
  (bind _returnvalue_2 (Utilities|String|Append "Resolution_test_" _returnvalue))
  (Math|Integer|IncrementInt (Variables|Default|GetResolutionIndex)
    (:%20%20
      (if (Utilities|Array|IsValidIndex _resolutions _resolutionindex)
        (Class|GameUserSettings|SetScreenResolution (stale EventInitializeTestRun _returnvalue_2) (Utilities|Array|Get(acopy) _resolutions _resolutionindex))
        (Class|GameUserSettings|ApplyResolutionSettings (stale EventInitializeTestRun _returnvalue_2) false)
        (Default|StartPerformanceProfiling (Variables|/SentinelAutomation/BP_BaseSentinelSettings.BP_BaseSentinelSettings_C|GetPerformanceComponent (Variables|Default|GetSettingsActor)) _returnvalue_2 _returnvalue_2)
        (else
          (CallFunction|FinishTestRunning))))))

(event EventInitializeTestRun
  (bind _returnvalue (Utilities|String|Append "Resolution_test_" "0"))
  (bind _settingsactor (Variables|Default|GetSettingsActor))
  (bind _performancecomponent (Variables|/SentinelAutomation/BP_BaseSentinelSettings.BP_BaseSentinelSettings_C|GetPerformanceComponent _settingsactor))
  (Utilities|FlowControl|Sequence
    (:then_0
      (bind _returnvalue_2 (Settings|GetGameUserSettings))
      (bind _resolutions (Class|KismetSystemLibrary|GetSupportedFullscreenResolutions))
      (Variables|Default|SetResolutions _resolutions))
    (:then_1
      (EventDispatchers|BindEventtoOnSingleScreenshotFinished _performancecomponent (delegate Custom|NextShot))
      (Default|StartPerformanceProfiling _performancecomponent _returnvalue _returnvalue))))

(fn ConstructionScript
  (|CallParentFunction))