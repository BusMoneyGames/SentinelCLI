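; Startup-map test settings Blueprint for Sentinel automated tests, choosing what runs based on the test configuration name.
; The Resolution Test gathers test locations and starts on them, Startup runs the parent's default behavior, and Asset Tests opens an asset review level.
; When a test finishes in the level, the Resolution Test defers to the parent to quit, while Startup chains into a second startup test level.
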(event EventStartTestConfiguuration
  (params (ConfigurationName :type String))
  (bind _output_get (Variables|Default|SetTestConfiguration ConfigurationName))
  (switch string _output_get
    (:sentinelTest_ResolutionTest
      (bind _outactors (CallFunction|GetTestLocations (Variables|Default|GetTestConfiguration)))
      (CallFunction|AddTestLocationsandStart _outactors))
    (:sentinelTest_Startup
      ;[1 1 1] Run the default behavior
      (|CallParentFunction (Variables|Default|GetTestConfiguration)))
    (:sentinelTest_AssetTests
      (Game|OpenLevel(byName) "Map_AssetReview02"))))

(event EventOnTestFinishedinLevel
  (switch string (Variables|Default|GetTestConfiguration)
    (:sentinelTest_ResolutionTest
      ;[1 1 1] Quit after the resolution test
      (|CallParentFunction))
    (:sentinelTest_Startup
      (Game|OpenLevel(byName) "Map_StartupTestSecondLevel"))))

(fn ConstructionScript
  (|CallParentFunction))